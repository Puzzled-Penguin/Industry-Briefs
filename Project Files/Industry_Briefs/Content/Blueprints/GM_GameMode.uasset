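; Game mode that runs a UI-driven shop with four factions whose values affect item pricing.
; On BeginPlay it switches to UI-only input with a visible cursor and adds the main and shop HUD widgets.
; CE_FactionChange adds a delta to the chosen faction's clamped value, prints it, then tells every shop item to update its price.
; Helper functions toggle between UI-only and game-and-UI input.
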(event `self.ReceiveBeginPlay`
  (`|ExecutionSequence`
    (:`then_0`
      (`self.UI Mode`))
    (:`then_1`
      (bind _returnvalue (`|CreateWidget` "/Game/Blueprints/UI/WD_HUD.WD_HUD_C"))
      (`UserWidget.AddToViewport` _returnvalue 1))
    (:`then_2`
      (bind _returnvalue_2 (`|CreateWidget` "/Game/Blueprints/UI/WD_ShopHUD.WD_ShopHUD_C"))
      (bind _output_get (set `self.ShopHud Ref` _returnvalue_2))
      (`UserWidget.AddToViewport` _output_get 0))))

(event `CE_FactionChange`
  (params (Faction :type "/Game/Blueprints/EN_Factions Enum" :default "NewEnumerator0") (Percentage :type "Float (double-precision)"))
  (switch `/Game/Blueprints/EN_Factions` Faction
    (:`NewEnumerator0`
      (set `self.True Sons` (`KismetMathLibrary.FClamp` (+ (`self.True Sons`) Percentage) 0.1 1000.0))
      (`KismetSystemLibrary.PrintString` (`KismetTextLibrary.Conv_TextToString` (`|FormatText` "True Sons {Faction} / {Change}" (`self.True Sons`) Percentage)) true true (struct :`R` 1.0 :`G` 0.259243 :`A` 1.0) 5.0))
    (:`NewEnumerator1`
      (set `self.Hyenas` (`KismetMathLibrary.FClamp` (+ (`self.Hyenas`) Percentage) 0.1 1000.0))
      (`KismetSystemLibrary.PrintString` (`KismetTextLibrary.Conv_TextToString` (`|FormatText` "Hyenas {Faction} / {Change}" (`self.Hyenas`) Percentage)) true true (struct :`R` 1.0 :`G` 0.259243 :`A` 1.0) 5.0))
    (:`NewEnumerator2`
      (set `self.Outcasts` (`KismetMathLibrary.FClamp` (+ (`self.Outcasts`) Percentage) 0.1 1000.0))
      (`KismetSystemLibrary.PrintString` (`KismetTextLibrary.Conv_TextToString` (`|FormatText` "Outcasts {Faction} / {Change}" (`self.Outcasts`) Percentage)) true true (struct :`R` 1.0 :`G` 0.259243 :`A` 1.0) 5.0))
    (:`NewEnumerator3`
      (set `self.Black Tusk` (`KismetMathLibrary.FClamp` (+ (`self.Black Tusk`) Percentage) 0.1 1000.0))
      (`KismetSystemLibrary.PrintString` (`KismetTextLibrary.Conv_TextToString` (`|FormatText` "Black Tusk {Faction} / {Change}" (`self.Black Tusk`) Percentage)) true true (struct :`R` 1.0 :`G` 0.259243 :`A` 1.0) 5.0)))
  (for _array_element (`/Game/Blueprints/UI/WD_ShopHUD.Items` (`self.ShopHud Ref`))
    (`/Game/Blueprints/UI/WD_ShopItem.CE_PriceChange` _array_element)))

(fn `Game Mode`
  (bind _returnvalue (`GameplayStatics.GetPlayerController` 0))
  (set `PlayerController.bShowMouseCursor` false _returnvalue)
  (set `PlayerController.bEnableClickEvents` false _returnvalue)
  (`WidgetBlueprintLibrary.SetInputMode_GameAndUIEx` _returnvalue null "DoNotLock" true true))

(fn `UI Mode`
  (bind _returnvalue (`GameplayStatics.GetPlayerController` 0))
  (set `PlayerController.bShowMouseCursor` true _returnvalue)
  (set `PlayerController.bEnableClickEvents` true _returnvalue)
  (`WidgetBlueprintLibrary.SetInputMode_UIOnlyEx` _returnvalue null "DoNotLock" true))

(fn `UserConstructionScript`)